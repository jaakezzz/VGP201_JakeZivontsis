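; BP_Gun is a gun Blueprint for an FPS, with stub functions that suggest a base for specific weapons.
; An interface-style shoot event forwards start and end positions to OnShoot, which is empty here.
; Getters expose the Damage, FireRate and Range variables, while GetClipSize returns a hardcoded zero instead of reading a variable.
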(event EventBeginPlay)

(event Collision|EventActorBeginOverlap
  (params (OtherActor :type Actor%20Object%20Reference)))

(event EventTick
  (params (DeltaSeconds :type Float%20%28single-precision%29)))

(event EventOnShootInterface
  (params (StartPosition :type Vector :default "0, 0, 0") (EndPosition :type Vector :default "0, 0, 0"))
  (CallFunction|OnShoot StartPosition EndPosition))

(fn ConstructionScript)

(fn OnShoot
  (params (StartPosition :type Vector) (EndPosition :type Vector)))

(fn GetClipSize
  (return 0))

(fn GetDamage
  (return (Variables|GunVar|GetDamage)))

(fn GetFireRate
  (return (Variables|GunVar|GetFireRate)))

(fn GetRange
  (return (Variables|GunVar|GetRange)))