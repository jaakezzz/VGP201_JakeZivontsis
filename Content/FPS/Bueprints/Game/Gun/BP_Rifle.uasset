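; Rifle weapon Blueprint that overrides its parent gun's OnShoot to fire a hitscan shot.
; After calling the parent, it line traces the Visibility channel between the given positions, ignoring the player character, and applies Damage to the hit actor through generic ApplyDamage.
; Debug strings and a drawn trace show each shot.
; An unconnected BP_Enemy cast calling TakeDamage never runs.
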(event EventBeginPlay)

(event Collision|EventActorBeginOverlap
  (params (OtherActor :type Actor%20Object%20Reference)))

(event EventTick
  (params (DeltaSeconds :type Float%20%28single-precision%29)))

(fn ConstructionScript
  (|CallParentFunction))

(fn OnShoot
  (params (StartPosition :type Vector :default "0, 0, 0") (EndPosition :type Vector :default "0, 0, 0"))
  (|CallParentFunction StartPosition EndPosition)
  (Development|PrintString "Firing Rifle")
  (bind _outhit (Collision|LineTraceByChannel StartPosition EndPosition "TraceTypeQuery1" false (Utilities|Array|MakeArray (Game|GetPlayerCharacter 0)) "ForDuration"))
  (Development|PrintString (Utilities|GetObjectName (.HitActor (Collision|BreakHitResult _outhit))))
  (Game|Damage|ApplyDamage (.HitActor (Collision|BreakHitResult _outhit)) (Variables|Default|GetDamage) 0 0))