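; AC_HealthComponent is an actor component that tracks an owner's health in the FPS game.
; On BeginPlay it calls Init to store the min and max bounds and start at full health.
; Heal and Damage apply absolute amounts through SetHealth, which clamps to those bounds.
; Getters expose current health, a 0–1 normalized value and a dead check at minimum health, all polled, with no events fired.
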(event EventBeginPlay
  (bind _maxhealth (Variables|Config|GetMaxHealth))
  (CallFunction|Init (Variables|Config|GetMinHealth) _maxhealth _maxhealth))

(event EventTick
  (params (DeltaSeconds :type Float%20%28single-precision%29)))

(fn GetHealth
  (return (Variables|Core|GetHealth)))

(fn SetHealth
  (params (NewHealth :type Float%20%28double-precision%29))
  (bind _output_get (Variables|Core|SetHealth (CallFunction|ClampHealth NewHealth)))
  (return _output_get))

(fn ClampHealth
  (params (Value :type Float%20%28double-precision%29))
  (return (Math|Float|Clamp(Float) Value (Variables|Config|GetMinHealth) (Variables|Config|GetMaxHealth))))

(fn Heal
  (params (HealValue :type Float%20%28double-precision%29))
  (CallFunction|SetHealth (+ (Math|Float|Absolute(Float) HealValue) (CallFunction|GetHealth))))

(fn Damage
  (params (DamageValue :type Float%20%28double-precision%29))
  (CallFunction|SetHealth (- (CallFunction|GetHealth) (Math|Float|Absolute(Float) DamageValue))))

(fn GetNormalizedHealth
  (return (Math|Float|Clamp(Float) (/ (CallFunction|GetHealth) (Variables|Config|GetMaxHealth)))))

(fn IsDead
  (return (<= (CallFunction|GetHealth) (Variables|Config|GetMinHealth))))

(fn Init
  (params (MinHealth :type Float%20%28double-precision%29) (MaxHealth :type Float%20%28double-precision%29) (StartingHealth :type Float%20%28double-precision%29))
  (Variables|Config|SetMinHealth MinHealth)
  (Variables|Config|SetMaxHealth MaxHealth)
  (CallFunction|SetHealth StartingHealth))