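; FPS game mode that owns the HUD, elapsed-time counter and score-based win condition.
; BeginPlay creates WBP_GameMenu, sets game-only input with a hidden cursor, then pushes initial timer and score to the widget.
; Tick calls IncrementTimer, whose one-second Delay throttles GameTimer increments and HUD refreshes.
; UpdateScore refreshes the displayed score and opens WinMap once Score reaches 24; Score is not modified here.
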(event EventBeginPlay
  (bind _returnvalue (Game|GetPlayerController 0))
  (Development|PrintString "Spawning BP_Gamemode" true true "(R=0.000000,G=0.660000,B=1.000000,A=1.000000)" 5.0) ; Debug: Gamemode init
  ;[0.15 0.15 0.15 0.5] Create HUD (GameMenu) and set input
  (bind _returnvalue_2 (UserInterface|CreateWidget "/Game/FPS/Bueprints/Game/GUI/WBP_GameMenu.WBP_GameMenu_C"))
  (bind _output_get (Variables|Config|SetGameMenuRef _returnvalue_2))
  (UserInterface|Viewport|AddtoViewport _output_get 0)
  (Input|SetInputModeGameOnly _returnvalue false)
  (Variables|/Script/Engine.PlayerController|SetbShowMouseCursor _returnvalue false)
  (CallFunction|UpdateHUDTimer)
  (CallFunction|UpdateScore))

(event EventTick
  (params (DeltaSeconds :type Float%20%28single-precision%29))
  (Utilities|IncrementTimer))

(fn ConstructionScript)

(fn UpdateHUDTimer
  (bind _aswbp_game_menu (Utilities|Casting|CastToWBP_GameMenu (Variables|Config|GetGameMenuRef)))
  (Default|UpdateTimer _aswbp_game_menu (Variables|Config|GetGameTimer)))

(fn UpdateScore
  (bind _aswbp_game_menu (Utilities|Casting|CastToWBP_GameMenu (Variables|Config|GetGameMenuRef)))
  (Default|UpdateScore _aswbp_game_menu (Variables|Config|GetScore))
  (if (>= (Variables|Config|GetScore) 24)
    (Game|OpenLevel(byObjectReference) "/Game/FPS/Maps/WinMap.WinMap")))